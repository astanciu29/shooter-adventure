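; Interactable sliding door whose Cube slides sideways along Y when the OpenDoor event runs, driven by a timeline lerp.
; A BP_DefaultCharacter entering the Box trigger plays a closing timeline and sets a flag that blocks later overlap replays.
; The closing lerp has a constant zero Alpha, so it holds the Cube at a partly open offset rather than animating it shut.
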(event OnComponentBeginOverlap(Box)
  (params (OverlappedComponent :type Primitive%20Component%20Object%20Reference) (OtherActor :type Actor%20Object%20Reference) (OtherComp :type Primitive%20Component%20Object%20Reference) (OtherBodyIndex :type Integer) (bFromSweep :type Boolean) (SweepResult :type Hit%20Result%20Structure%20%28by%20ref%29))
  (Utilities|Casting|CastToBP_DefaultCharacter OtherActor)
  (if (not (Variables|Default|GetHasPlayedGoneThroughDoor))
    (Timeline|ClosingDoorTimeline Play
      (:Update
        (Transformation|SetRelativeLocation (Variables|Default|GetCube) (Math|Vector|Lerp(Vector) "0,-70.000000,150.000000" "0,0.000000,150.000000" 0.0) false false)
        (Variables|Default|SetHasPlayedGoneThroughDoor true)))))

(event Custom|OpenDoor
  (bind _doortrack (Timeline|OpenDoorTimeline Play)
    (:Update
      (Transformation|SetRelativeLocation (Variables|Default|GetCube) (Math|Vector|Lerp(Vector) "0, 0,150.000000" "0,-180.000000,150.000000" _doortrack) false false))))

(event EventBeginPlay)

(fn ConstructionScript)